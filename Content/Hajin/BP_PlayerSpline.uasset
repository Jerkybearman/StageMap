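; BP_PlayerSpline controls the player's camera zoom by driving the length of a spring arm.
; On BeginPlay it sets a close goal length, then after a short delay switches to the farthest one, producing an opening pull-out.
; Scroll input adjusts the goal within those limits and prints it.
; Tick eases the arm toward the goal with FInterpTo; no spline logic appears in the graphs.
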(event `self.ReceiveBeginPlay`
  (set `self.Goal Arm Length` 500.0)
  (`KismetSystemLibrary.Delay` 2.0)
  (set `self.Goal Arm Length` 12775.0))

(event `EnhancedInput|/Game/Hajin/Camera/CameraInput/Action/IA_Scroll`
  (params (ActionValue :type "Float (double-precision)") (ElapsedSeconds :type "Float (double-precision)") (TriggeredSeconds :type "Float (double-precision)") (InputAction :type "InputAction Object Reference" :default "/Game/Hajin/Camera/CameraInput/Action/IA_Scroll.IA_Scroll"))
  (:`Triggered`
    (bind _output_get (set `self.Goal Arm Length` (`KismetMathLibrary.FClamp` (+ (`self.Goal Arm Length`) (* ActionValue (`self.ScrollSpeed`))) 500.0 12775.0)))
    (`KismetSystemLibrary.PrintString` (`KismetStringLibrary.Conv_DoubleToString` _output_get))))

(event `self.ReceiveTick`
  (params (DeltaSeconds :type "Float (single-precision)"))
  (set `SpringArmComponent.TargetArmLength` (`KismetMathLibrary.FInterpTo` (`SpringArmComponent.TargetArmLength` (`self.SpringArm`)) (`self.Goal Arm Length`) DeltaSeconds 7.5) (`self.SpringArm`)))

(fn `UserConstructionScript`)